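; BP_MenuGameMode is the game mode for the main menu, creating WBP_MainMenu and adding it to the viewport on BeginPlay.
; It also relays selection previews: UpdateMapImage and UpdateVehicleImage pass track and vehicle images to the SelectGameMenu widget when that reference is valid.
; SelectGameMenu is not assigned within this Blueprint.
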(event `self.ReceiveBeginPlay`
  (bind _returnvalue (`|CreateWidget` "/Game/UI/Widgets/MainMenu/WBP_MainMenu.WBP_MainMenu_C"))
  (`UserWidget.AddToViewport` _returnvalue 0))

(event `self.UpdateMapImage`
  (params (MapImage :type "Texture2D Object Reference"))
  (bind _selectgamemenu (`self.SelectGameMenu`))
  (if (`KismetSystemLibrary.IsValid` _selectgamemenu)
    (`/Game/UI/Widgets/MainMenu/WBP_SelectGame.SetTrackImage` _selectgamemenu MapImage)))

(event `self.UpdateVehicleImage`
  (params (VehicleImage :type "Texture2D Object Reference"))
  (bind _selectgamemenu (`self.SelectGameMenu`))
  (if (`KismetSystemLibrary.IsValid` _selectgamemenu)
    (`/Game/UI/Widgets/MainMenu/WBP_SelectGame.SetVehicleImage` _selectgamemenu VehicleImage)))

(fn `UserConstructionScript`)